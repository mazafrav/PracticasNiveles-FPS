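; NPC Blueprint that shows a floating text label when the player comes within talking distance.
; Every Tick, it rotates the TextRender to face the player camera and compares its distance to the FirstPersonCharacter's TalkingDistance.
; In range, it makes the text visible and a Delay of ShowTime hides it again, with Tick re-showing it while the player stays close.
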(event `self.ReceiveBeginPlay`
  (`SceneComponent.SetVisibility` (`self.TextRender`) false true))

(event `self.ReceiveTick`
  (params (DeltaSeconds :type "Float (single-precision)"))
  (`|ExecutionSequence`
    (:`then_0`
      (`SceneComponent.K2_SetWorldRotation` (`self.TextRender`) (`KismetMathLibrary.FindLookAtRotation` (`self.K2_GetActorLocation`) (`self.K2_GetActorLocation` (`GameplayStatics.GetPlayerCameraManager` 0))) false false))
    (:`then_1`
      (bind _asfirst_person_character (cast `/Game/Blueprints/FirstPersonCharacter` (`GameplayStatics.GetPlayerPawn` 0)))
      (if (<= (`self.GetDistanceTo` _asfirst_person_character) (`/Game/Blueprints/FirstPersonCharacter.Talking distance` _asfirst_person_character))
        (`SceneComponent.SetVisibility` (`self.TextRender`) true true)
        (`KismetSystemLibrary.Delay` (`self.Show time`))
        (`SceneComponent.SetVisibility` (`self.TextRender`) false true)))))

(fn `UserConstructionScript`)